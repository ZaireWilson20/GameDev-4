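; Player Blueprint that controls the active falling block in a 3D Tetris-style game, fed by a Spawner.
; Tick moves the block down by a drop vector, which speeds up while Drop is held.
; Directional inputs shift it one grid cell horizontally when its bound counters and side triggers allow, updating those counters.
; BeginPlay requests the first block, ChangeBlock swaps the controlled one, and G resets the Spawner's bag.
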(event Custom|ChangeBlock
  (params (NewBlock :type Items%20Blueprint%20Object%20Reference))
  ;[1 1 1] Change Block
  (Variables|Default|Setblock NewBlock))

(event EventBeginPlay
  ;[1 1 1] Init
  (Input|EnableInput (Game|GetPlayerController 0))
  (Variables|Default|Setdrop_vector "0,0.000000,-100.000000")
  (Default|SpawnNext (Variables|Default|GetSpawner)))

(event EventTick
  (params (DeltaSeconds :type Float%20%28single-precision%29))
  (bind _block (Variables|Default|Getblock))
  ;[1 1 1] Move Active Block Down Every Tick
  (if (not (== _block (Variables|/Game/Blueprints/Spawn_Blueprint.Spawn_Blueprint_C|Getnull_block (Variables|Default|GetSpawner))))
    (Transformation|AddActorLocalOffset _block (* (Variables|Default|Getdrop_vector) (Math|Conversions|ToVector(Float) DeltaSeconds)) false false)))

(event Input|ActionEvents|InputActionLeft
  (params (Key :type Key%20Structure))
  (bind _block (Variables|Default|Getblock))
  ;[1 1 1] Control Block Position TODO: Check if block is null
  (:Pressed
    (if (not (== (Variables|/Game/Blueprints/Items_Blueprint.Items_Blueprint_C|GetLeftBound _block) 0))
      (if (== (Variables|/Game/Blueprints/Items_Blueprint.Items_Blueprint_C|GetLeftTrigger _block) 0)
        (Transformation|AddActorLocalOffset _block "-100.000000, 0, 0" false false)
        (Variables|/Game/Blueprints/Items_Blueprint.Items_Blueprint_C|SetLeftBound _block (+ (Variables|/Game/Blueprints/Items_Blueprint.Items_Blueprint_C|GetLeftBound _block) -1))
        (Variables|/Game/Blueprints/Items_Blueprint.Items_Blueprint_C|SetRightBound _block (+ (Variables|/Game/Blueprints/Items_Blueprint.Items_Blueprint_C|GetRightBound _block) -1))))))

(event Input|ActionEvents|InputActionRight
  (params (Key :type Key%20Structure))
  (bind _block (Variables|Default|Getblock))
  ;[1 1 1] Control Block Position TODO: Check if block is null
  (:Pressed
    (if (not (== (Variables|/Game/Blueprints/Items_Blueprint.Items_Blueprint_C|GetRightBound _block) 4))
      (if (== (Variables|/Game/Blueprints/Items_Blueprint.Items_Blueprint_C|GetRightTrigger _block) 0)
        (Transformation|AddActorLocalOffset _block "100.000000, 0, 0" false false)
        (Variables|/Game/Blueprints/Items_Blueprint.Items_Blueprint_C|SetRightBound _block (+ (Variables|/Game/Blueprints/Items_Blueprint.Items_Blueprint_C|GetRightBound _block) 1))
        (Variables|/Game/Blueprints/Items_Blueprint.Items_Blueprint_C|SetLeftBound _block (+ (Variables|/Game/Blueprints/Items_Blueprint.Items_Blueprint_C|GetLeftBound _block) 1))))))

(event Input|ActionEvents|InputActionDown
  (params (Key :type Key%20Structure))
  (bind _block (Variables|Default|Getblock))
  ;[1 1 1] Control Block Position TODO: Check if block is null
  (:Pressed
    (if (not (== (Variables|/Game/Blueprints/Items_Blueprint.Items_Blueprint_C|GetBottomBound _block) 0))
      (if (== (Variables|/Game/Blueprints/Items_Blueprint.Items_Blueprint_C|GetBottomTrigger _block) 0)
        (Transformation|AddActorLocalOffset _block "0.000000,100.000000, 0" false false)
        (Variables|/Game/Blueprints/Items_Blueprint.Items_Blueprint_C|SetBottomBound _block (+ (Variables|/Game/Blueprints/Items_Blueprint.Items_Blueprint_C|GetBottomBound _block) -1))
        (Variables|/Game/Blueprints/Items_Blueprint.Items_Blueprint_C|SetTopBound _block (+ (Variables|/Game/Blueprints/Items_Blueprint.Items_Blueprint_C|GetTopBound _block) -1))))))

(event Input|ActionEvents|InputActionUp
  (params (Key :type Key%20Structure))
  (bind _block (Variables|Default|Getblock))
  ;[1 1 1] Control Block Position TODO: Check if block is null
  (:Pressed
    (if (not (== (Variables|/Game/Blueprints/Items_Blueprint.Items_Blueprint_C|GetTopBound _block) 4))
      (if (== (Variables|/Game/Blueprints/Items_Blueprint.Items_Blueprint_C|GetTopTrigger _block) 0)
        (Transformation|AddActorLocalOffset _block "0.000000,-100.000000, 0" false false)
        (Variables|/Game/Blueprints/Items_Blueprint.Items_Blueprint_C|SetTopBound _block (+ (Variables|/Game/Blueprints/Items_Blueprint.Items_Blueprint_C|GetTopBound _block) 1))
        (Variables|/Game/Blueprints/Items_Blueprint.Items_Blueprint_C|SetBottomBound _block (+ (Variables|/Game/Blueprints/Items_Blueprint.Items_Blueprint_C|GetBottomBound _block) 1))))))

(event Input|ActionEvents|InputActionDrop
  (params (Key :type Key%20Structure))
  ;[1 1 1] Control Drop Speed
  (:Pressed
    (Variables|Default|Setdrop_vector "0, 0,-500.000000"))
  (:Released
    (Variables|Default|Setdrop_vector "0, 0,-100.000000")))

(event Input|KeyboardEvents|G
  (params (Key :type Key%20Structure))
  ;[1 1 1] Reset Bag
  (:Pressed
    (Default|ResetBag (Variables|Default|GetSpawner))))

(fn ConstructionScript)