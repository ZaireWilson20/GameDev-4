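; Item block actor of configurable size with weight and durability, which asks its Spawner for the next block when stopped.
; SetUp attaches a grid of ItemHitbox actors, offsets even dimensions, computes movement bounds and sizes the side boxes, but zeroes Weight and Durability despite its parameters.
; Side-box overlaps maintain per-side trigger counters.
; Hitbox hits split Weight across an incrementing active count; durability damage has no lose condition yet.
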(event OnComponentBeginOverlap(BottomSidebox)
  (params (OverlappedComponent :type Primitive%20Component%20Object%20Reference) (OtherActor :type Actor%20Object%20Reference) (OtherComp :type Primitive%20Component%20Object%20Reference) (OtherBodyIndex :type Integer) (bFromSweep :type Boolean) (SweepResult :type Hit%20Result%20Structure%20%28by%20ref%29))
  ;[1 1 1] Bottom Sidebox Overlap
  (if (not (== OtherActor self))
    (Variables|Default|SetBottomTrigger (+ (Variables|Default|GetBottomTrigger) 1))))

(event OnComponentEndOverlap(BottomSidebox)
  (params (OverlappedComponent :type Primitive%20Component%20Object%20Reference) (OtherActor :type Actor%20Object%20Reference) (OtherComp :type Primitive%20Component%20Object%20Reference) (OtherBodyIndex :type Integer))
  ;[1 1 1] Bottom Sidebox Overlap
  (if (not (== OverlappedComponent self))
    (Variables|Default|SetBottomTrigger (+ (Variables|Default|GetBottomTrigger) -1))))

(event OnComponentBeginOverlap(TopSidebox)
  (params (OverlappedComponent :type Primitive%20Component%20Object%20Reference) (OtherActor :type Actor%20Object%20Reference) (OtherComp :type Primitive%20Component%20Object%20Reference) (OtherBodyIndex :type Integer) (bFromSweep :type Boolean) (SweepResult :type Hit%20Result%20Structure%20%28by%20ref%29))
  ;[1 1 1] Top Sidebox Overlap
  (if (not (== OtherActor self))
    (Variables|Default|SetTopTrigger (+ (Variables|Default|GetTopTrigger) 1))))

(event OnComponentEndOverlap(TopSidebox)
  (params (OverlappedComponent :type Primitive%20Component%20Object%20Reference) (OtherActor :type Actor%20Object%20Reference) (OtherComp :type Primitive%20Component%20Object%20Reference) (OtherBodyIndex :type Integer))
  ;[1 1 1] Top Sidebox Overlap
  (if (not (== OtherActor self))
    (Variables|Default|SetTopTrigger (+ (Variables|Default|GetTopTrigger) -1))))

(event OnComponentBeginOverlap(RightSidebox)
  (params (OverlappedComponent :type Primitive%20Component%20Object%20Reference) (OtherActor :type Actor%20Object%20Reference) (OtherComp :type Primitive%20Component%20Object%20Reference) (OtherBodyIndex :type Integer) (bFromSweep :type Boolean) (SweepResult :type Hit%20Result%20Structure%20%28by%20ref%29))
  ;[1 1 1] Right Sidebox Overlap
  (if (not (== OtherActor self))
    (Variables|Default|SetRightTrigger (+ (Variables|Default|GetRightTrigger) 1))))

(event OnComponentEndOverlap(RightSidebox)
  (params (OverlappedComponent :type Primitive%20Component%20Object%20Reference) (OtherActor :type Actor%20Object%20Reference) (OtherComp :type Primitive%20Component%20Object%20Reference) (OtherBodyIndex :type Integer))
  ;[1 1 1] Right Sidebox Overlap
  (if (not (== OtherActor self))
    (Variables|Default|SetRightTrigger (+ (Variables|Default|GetRightTrigger) -1))))

(event OnComponentBeginOverlap(LeftSidebox)
  (params (OverlappedComponent :type Primitive%20Component%20Object%20Reference) (OtherActor :type Actor%20Object%20Reference) (OtherComp :type Primitive%20Component%20Object%20Reference) (OtherBodyIndex :type Integer) (bFromSweep :type Boolean) (SweepResult :type Hit%20Result%20Structure%20%28by%20ref%29))
  ;[1 1 1] Left Sidebox Overlap
  (if (not (== OtherActor self))
    (Variables|Default|SetLeftTrigger (+ (Variables|Default|GetLeftTrigger) 1))))

(event OnComponentEndOverlap(LeftSidebox)
  (params (OverlappedComponent :type Primitive%20Component%20Object%20Reference) (OtherActor :type Actor%20Object%20Reference) (OtherComp :type Primitive%20Component%20Object%20Reference) (OtherBodyIndex :type Integer))
  ;[1 1 1] Left Sidebox Overlap
  (if (not (== OtherActor self))
    (Variables|Default|SetLeftTrigger (+ (Variables|Default|GetLeftTrigger) -1))))

(event Custom|HitboxHitSomething
  ;[1 1 1] Updates Weight Distribution
  (bind _result (Math|Integer|IncrementInt (Variables|Default|GetNumActiveHitBoxes))
    (:%20%20
      (for _array_element (Variables|Default|GetItemHitBoxes)
        (bind _asitem_hitbox_blueprint (Utilities|Casting|CastToItemHitbox_Blueprint _array_element))
        (Default|ApplyWeight _asitem_hitbox_blueprint (/ (Variables|Default|GetWeight) (Math|Conversions|ToFloat(Integer) _result)))))))

(event Custom|ReduceDurability
  (params (Reduce :type Float%20%28single-precision%29))
  ;[1 1 1] Take Durability Dmg TODO: Add lose condition
  (Variables|Default|SetDurability (- (Variables|Default|GetDurability) Reduce)))

(event Custom|StopBlock
  ;[1 1 1] Stop Block TODO: Tell spawner to spawn new block, and set that to be controlled
  (Default|SpawnNext (Variables|Default|GetSpawner)))

(fn ConstructionScript)

(fn SetUp
  (params (NewWidth :type Integer) (NewLength :type Integer) (NewHeight :type Integer) (NewWeight :type Float%20%28single-precision%29) (NewDurability :type Float%20%28single-precision%29))
  (bind _self self)
  (bind _topsidebox (Variables|Default|GetTopSidebox))
  (bind _bottomsidebox (Variables|Default|GetBottomSidebox))
  (bind _leftsidebox (Variables|Default|GetLeftSidebox))
  (bind _rightsidebox (Variables|Default|GetRightSidebox))
  ;[1 1 1] Init Vars
  (Variables|Default|SetWidth NewWidth)
  (Variables|Default|SetLength NewLength)
  (Variables|Default|SetHeight NewHeight)
  (Variables|Default|SetWeight 0.0)
  (Variables|Default|SetDurability 0.0)
  ;[1 1 1] Create Hitboxes
  (Transformation|SetActorLocation "0.000000,0.000000,600.000000" false true)
  (for _index (range 1 NewWidth)
    (for _index_2 (range 1 NewLength)
      (bind _returnvalue (Game|SpawnActorfromClass "/Game/Blueprints/ItemHitbox_Blueprint.ItemHitbox_Blueprint_C" (Math|Conversions|ToTransform(Vector) (Math|Vector|MakeVector (Math|Conversions|ToFloat(Integer) (- (* 50 (Variables|Default|GetWidth)) (* 100 _index))) (Math|Conversions|ToFloat(Integer) (- (* 50 (Variables|Default|GetLength)) (* 100 _index_2))) (Math|Conversions|ToFloat(Integer) (* -50 (Variables|Default|GetHeight))))) "AlwaysSpawn" 0 0)) ; remember to set class to spawn
      (Utilities|Array|Add (Variables|Default|GetItemHitBoxes) _returnvalue)
      (Variables|/Game/Blueprints/ItemHitbox_Blueprint.ItemHitbox_Blueprint_C|SetItem _returnvalue _self)
      (Transformation|AttachActorToActor _returnvalue _self "None" "KeepRelative" "KeepRelative" "KeepRelative" false)))
  ;[1 1 1] Setup Item Position
  (Transformation|SetActorLocation "0.000000,0.000000,600.000000" false true)
  (if (> (Math|Integer|%(Integer) (Variables|Default|GetWidth) 2) 0)
    _
    (else
      (Transformation|AddActorLocalOffset "50.000000, 0, 0" false true)))
  (if (> (Math|Integer|%(Integer) (Variables|Default|GetLength) 2) 0)
    _
    (else
      (Transformation|AddActorLocalOffset "0.000000,50.000000, 0" false true)))
  (if (> (Math|Integer|%(Integer) (Variables|Default|GetHeight) 2) 0)
    _
    (else
      (Transformation|AddActorLocalOffset "0.000000,0.000000,50.000000" false true)))
  ;[1 1 1] SetRightBound
  (if (> (Math|Integer|%(Integer) (Variables|Default|GetWidth) 2) 0)
    (Variables|Default|SetRightBound (+ (/ (- (Variables|Default|GetWidth) 1) 2) 2))
    (else
      (Variables|Default|SetRightBound (+ (/ (Variables|Default|GetWidth) 2) 2))))
  ;[1 1 1] SetLeftBound
  (if (> (Math|Integer|%(Integer) (Variables|Default|GetWidth) 2) 0)
    (Variables|Default|SetLeftBound (- 2 (/ (- (Variables|Default|GetWidth) 1) 2)))
    (else
      (Variables|Default|SetLeftBound (- 2 (- (/ (Variables|Default|GetWidth) 2) 1)))))
  ;[1 1 1] SetTopBound
  (if (> (Math|Integer|%(Integer) (Variables|Default|GetLength) 2) 0)
    (Variables|Default|SetTopBound (+ (/ (- (Variables|Default|GetLength) 1) 2) 2))
    (else
      (Variables|Default|SetTopBound (+ (/ (Variables|Default|GetLength) 2) 2))))
  ;[1 1 1] SetBottomBound
  (if (> (Math|Integer|%(Integer) (Variables|Default|GetLength) 2) 0)
    (Variables|Default|SetBottomBound (- 2 (/ (- (Variables|Default|GetLength) 1) 2)))
    (else
      (Variables|Default|SetBottomBound (- 2 (- (/ (Variables|Default|GetLength) 2) 1)))))
  ;[1 1 1] Setup Sideboxes
  (Transformation|SetRelativeScale3D _topsidebox (Math|Vector|MakeVector (Math|Conversions|ToFloat(Integer) (Variables|Default|GetLength)) (Math|Conversions|ToFloat(Integer) (Variables|Default|GetWidth)) (Math|Conversions|ToFloat(Integer) (Variables|Default|GetHeight))))
  (Class|SceneComponent|AddLocalTransform _topsidebox (Math|Conversions|ToTransform(Vector) (Math|Vector|MakeVector (* (- (Math|Conversions|ToFloat(Integer) (Variables|Default|GetLength)) 1.0) 5e+01) 0.0 0.0)) false true)
  (Transformation|SetRelativeScale3D _bottomsidebox (Math|Vector|MakeVector (Math|Conversions|ToFloat(Integer) (Variables|Default|GetLength)) (Math|Conversions|ToFloat(Integer) (Variables|Default|GetWidth)) (Math|Conversions|ToFloat(Integer) (Variables|Default|GetHeight))))
  (Class|SceneComponent|AddLocalTransform _bottomsidebox (Math|Conversions|ToTransform(Vector) (Math|Vector|MakeVector (* (- (Math|Conversions|ToFloat(Integer) (Variables|Default|GetLength)) 1.0) -5e+01) 0.0 0.0)) false true)
  (Transformation|SetRelativeScale3D _rightsidebox (Math|Vector|MakeVector (Math|Conversions|ToFloat(Integer) (Variables|Default|GetLength)) (Math|Conversions|ToFloat(Integer) (Variables|Default|GetWidth)) (Math|Conversions|ToFloat(Integer) (Variables|Default|GetHeight))))
  (Class|SceneComponent|AddLocalTransform _rightsidebox (Math|Conversions|ToTransform(Vector) (Math|Vector|MakeVector 0.0 (* (- (Math|Conversions|ToFloat(Integer) (Variables|Default|GetWidth)) 1.0) 5e+01) 0.0)) false true)
  (Transformation|SetRelativeScale3D _leftsidebox (Math|Vector|MakeVector (Math|Conversions|ToFloat(Integer) (Variables|Default|GetLength)) (Math|Conversions|ToFloat(Integer) (Variables|Default|GetWidth)) (Math|Conversions|ToFloat(Integer) (Variables|Default|GetHeight))))
  (Class|SceneComponent|AddLocalTransform _leftsidebox (Math|Conversions|ToTransform(Vector) (Math|Vector|MakeVector 0.0 (* (- (Math|Conversions|ToFloat(Integer) (Variables|Default|GetWidth)) 1.0) -5e+01) 0.0)) false true)
  (Transformation|SetRelativeScale3D (Variables|Default|GetCenterBox) (Math|Vector|MakeVector (Math|Conversions|ToFloat(Integer) (Variables|Default|GetLength)) (Math|Conversions|ToFloat(Integer) (Variables|Default|GetWidth)) (Math|Conversions|ToFloat(Integer) (Variables|Default|GetHeight)))))