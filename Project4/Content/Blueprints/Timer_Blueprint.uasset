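; Countdown timer Blueprint that shows the remaining seconds on screen, starting from 60.
; BeginPlay creates the Timer widget, adds it to the viewport and writes the starting Time to its text block.
; Tick uses a one-second Delay as a throttle to decrement Time and refresh the text.
; The count has no stop or action at zero.
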(event EventBeginPlay
  (bind _output_get (Variables|Default|SetTime 60))
  (bind _returnvalue (UserInterface|CreateWidget "/Game/Blueprints/Timer.Timer_C"))
  (Variables|Default|Settimer _returnvalue)
  (UserInterface|Viewport|AddtoViewport _returnvalue 0)
  (Rendering|Components|TextRender|SetText (Variables|/Game/Blueprints/Timer.Timer_C|GetTextBlock_98 _returnvalue) (Utilities|Text|ToText(Integer) _output_get)))

(event EventTick
  (params (DeltaSeconds :type Float%20%28single-precision%29))
  (Utilities|FlowControl|Delay 1.0)
  (bind _output_get (Variables|Default|SetTime (- (Variables|Default|GetTime) 1)))
  (Rendering|Components|TextRender|SetText (Variables|/Game/Blueprints/Timer.Timer_C|GetTextBlock_98 (Variables|Default|Gettimer)) (Utilities|Text|ToText(Integer) _output_get)))