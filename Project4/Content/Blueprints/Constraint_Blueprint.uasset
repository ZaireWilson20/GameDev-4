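; Constraint Blueprint that tests one placement or condition rule against the items in SpawnBlueprint's ItemArray.
; CheckItems branches on ConstraintType and returns true on a match: named item beneath another, named item below half durability, or heavier item atop a lighter one.
; The group rule compares the named item's count against a set of unique same-named items found beneath them.
; Stacking relationships come from each item's hitboxes via ItemBelow.
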(event EventBeginPlay)

(event EventTick
  (params (DeltaSeconds :type Float%20%28single-precision%29)))

(fn CheckItems
  (bind _constraint_type (Variables|Default|Getconstraint_type))
  ;[1 1 1] Branch on Constraint Type
  (if (Utilities|Enum|Equal(Enum) _constraint_type "top")
    ;[1 1 1] Look at all items below and return false if any of them match the item name
    (for _array_element (Variables|/Game/Blueprints/Spawn_Blueprint.Spawn_Blueprint_C|GetitemArray (Variables|Default|GetSpawnBlueprint))
      (bind _asitems_blueprint (Utilities|Casting|CastToItems_Blueprint _array_element))
      (for _array_element_2 (Variables|/Game/Blueprints/Items_Blueprint.Items_Blueprint_C|GetItemHitBoxes _asitems_blueprint)
        (if (Utilities|Enum|Equal(Enum) (Variables|/Game/Blueprints/Items_Blueprint.Items_Blueprint_C|GetName (Variables|/Game/Blueprints/ItemHitbox_Blueprint.ItemHitbox_Blueprint_C|GetItemBelow _array_element_2)) (Variables|Default|Getitem_name))
          (return true))))
    (return false)
    (elif (Utilities|Enum|Equal(Enum) _constraint_type "group")
      ;[1 1 1] Grouping constraint
      (Variables|Default|Setcounter 0)
      (Variables|Default|Settemp_items (Utilities|Set|MakeSet 0))
      (for _array_element_3 (Variables|/Game/Blueprints/Spawn_Blueprint.Spawn_Blueprint_C|GetitemArray (Variables|Default|GetSpawnBlueprint))
        (bind _asitems_blueprint_2 (Utilities|Casting|CastToItems_Blueprint _array_element_3))
        (if (Utilities|Enum|Equal(Enum) (Variables|/Game/Blueprints/Items_Blueprint.Items_Blueprint_C|GetName _asitems_blueprint_2) (Variables|Default|Getitem_name))
          (Variables|Default|Setcounter (+ (Variables|Default|Getcounter) 1))
          (bind _array_element_4 (Utilities|Array|ForEachLoopwithBreak (Variables|/Game/Blueprints/Items_Blueprint.Items_Blueprint_C|GetItemHitBoxes _asitems_blueprint_2))
            (:LoopBody
              (if (Utilities|Enum|Equal(Enum) (Variables|/Game/Blueprints/Items_Blueprint.Items_Blueprint_C|GetName (Variables|/Game/Blueprints/ItemHitbox_Blueprint.ItemHitbox_Blueprint_C|GetItemBelow _array_element_4)) (Variables|Default|Getitem_name))
                (if (not (Utilities|Set|Contains (Variables|Default|Gettemp_items) (Variables|/Game/Blueprints/ItemHitbox_Blueprint.ItemHitbox_Blueprint_C|GetItemBelow _array_element_4)))
                  (Utilities|Set|Add (Variables|Default|Gettemp_items) (Variables|/Game/Blueprints/ItemHitbox_Blueprint.ItemHitbox_Blueprint_C|GetItemBelow _array_element_4))))))))
      (if (< (Variables|Default|Getcounter) (- (Utilities|Set|Length (Variables|Default|Gettemp_items)) 1))
        (return true)
        (else
          (return false)))
      (elif (Utilities|Enum|Equal(Enum) _constraint_type "durability")
        ;[1 1 1] 50% durability
        (for _array_element_5 (Variables|/Game/Blueprints/Spawn_Blueprint.Spawn_Blueprint_C|GetitemArray (Variables|Default|GetSpawnBlueprint))
          (bind _asitems_blueprint_3 (Utilities|Casting|CastToItems_Blueprint _array_element_5))
          (if (Utilities|Enum|Equal(Enum) (Variables|/Game/Blueprints/Items_Blueprint.Items_Blueprint_C|GetName _asitems_blueprint_3) (Variables|Default|Getitem_name))
            (if (< (Variables|/Game/Blueprints/Items_Blueprint.Items_Blueprint_C|GetDurability _asitems_blueprint_3) (/ (Variables|/Game/Blueprints/Items_Blueprint.Items_Blueprint_C|GetMaxDurability _asitems_blueprint_3) 2.0))
              (return true))))
        (return false)
        (elif (Utilities|Enum|Equal(Enum) _constraint_type "weight_order")
          ;[1 1 1] Item weight stcking
          (for _array_element_6 (Variables|/Game/Blueprints/Spawn_Blueprint.Spawn_Blueprint_C|GetitemArray (Variables|Default|GetSpawnBlueprint))
            (bind _asitems_blueprint_4 (Utilities|Casting|CastToItems_Blueprint _array_element_6))
            (bind _array_element_7 (Utilities|Array|ForEachLoopwithBreak (Variables|/Game/Blueprints/Items_Blueprint.Items_Blueprint_C|GetItemHitBoxes _asitems_blueprint_4))
              (:LoopBody
                (if (> (Variables|/Game/Blueprints/Items_Blueprint.Items_Blueprint_C|GetWeight _asitems_blueprint_4) (Variables|/Game/Blueprints/Items_Blueprint.Items_Blueprint_C|GetWeight (Variables|/Game/Blueprints/ItemHitbox_Blueprint.ItemHitbox_Blueprint_C|GetItemBelow _array_element_7)))
                  (return true)))))
          (return false))))))