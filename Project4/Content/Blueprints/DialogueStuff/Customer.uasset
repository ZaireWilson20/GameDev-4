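; Customer Blueprint that issues a series of up to three timed Yes/No demands to the player through dialogue and demand widgets.
; Accepting adds a Constraint component configured from indexed item and type arrays; refusing deducts time from the spawner's timer.
; CheckConstraints runs each stored constraint's item check and triggers the spawner's game over on a true result.
; Tick's warning never fires, and some response and constraint-checking logic is left disconnected.
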(event Custom|Customer%20Start
  (Input|EnableInput (Game|GetPlayerController 0))
  (Utilities|FlowControl|Delay 1e+01)
  (CallFunction|GiveDemand))

(event Custom|give%20demand
  (Variables|Default|SetwaitingForResponse true)
  (Development|PrintString "bitchhh")
  (bind _returnvalue (UserInterface|CreateWidget "/Game/Blueprints/DialogueStuff/Dialogue.Dialogue_C" (Game|GetPlayerController 0)))
  (bind _output_get (Variables|Default|SetdialogueWidg _returnvalue))
  (UserInterface|Viewport|AddtoViewport _output_get 0)
  (Variables|/Game/Blueprints/DialogueStuff/Dialogue.Dialogue_C|SetDialougeText (Variables|Default|GetdialogueWidg) (Utilities|Text|ToText(String) (Utilities|String|Append (Utilities|String|ToString(Text) (Utilities|Array|Get(acopy) (Variables|Default|GetcustText) (Variables|Default|Getindex))) "    Q: Yes E: No")))
  (bind _returnvalue_2 (UserInterface|CreateWidget "/Game/Blueprints/CustomerDemands.CustomerDemands_C" (Game|GetPlayerController 0)))
  (bind _output_get_2 (Variables|Default|SetDemands _returnvalue_2))
  (UserInterface|Viewport|AddtoViewport _output_get_2 0)
  (Variables|/Game/Blueprints/CustomerDemands.CustomerDemands_C|SetdemandText _output_get_2 (Variables|Default|GetdemandText)))

(event EventTick
  (params (DeltaSeconds :type Float%20%28single-precision%29))
  (Variables|Default|SetconstraintStatus true)
  (if (not (Variables|Default|GetconstraintStatus))
    (Development|PrintString "WHY U IGNIORIN ME")))

(event Input|ActionEvents|InputActionYes
  (params (Key :type Key%20Structure))
  (:Pressed
    (if (Variables|Default|GetwaitingForResponse)
      (Development|PrintString "Hello")
      (bind _returnvalue (AddComponent|AddConstraintBlueprint))
      (Utilities|Array|Add (Variables|Default|Getconsts) _returnvalue)
      (Variables|/Game/Blueprints/Constraint_Blueprint.Constraint_Blueprint_C|SetSpawnBlueprint _returnvalue (Variables|Default|Getspawnboi))
      (Variables|/Game/Blueprints/Constraint_Blueprint.Constraint_Blueprint_C|Setitem_name _returnvalue (Utilities|String|ToString(Text) (Utilities|Array|Get(acopy) (Variables|Default|GetconstraintItem) (Variables|Default|Getindex))))
      (Variables|/Game/Blueprints/Constraint_Blueprint.Constraint_Blueprint_C|Setconstraint_type _returnvalue (Utilities|String|ToString(Text) (Utilities|Array|Get(acopy) (Variables|Default|GetconstraintType) (Variables|Default|Getindex))))
      (Widget|RemovefromParent (Variables|Default|GetdialogueWidg))
      (bind _output_get (Variables|Default|Setindex (+ (Variables|Default|Getindex) 1)))
      (Variables|Default|SetwaitingForResponse false)
      (if (< _output_get 3)
        (Utilities|FlowControl|Delay 1e+01)
        (CallFunction|GiveDemand)))))

(event Input|ActionEvents|InputActionNo
  (params (Key :type Key%20Structure))
  (bind _spawnboi (Variables|Default|Getspawnboi))
  (bind _timer_blueprint (Variables|/Game/Blueprints/Spawn_Blueprint.Spawn_Blueprint_C|GetTimer_Blueprint _spawnboi))
  (:Pressed
    (if (Variables|Default|GetwaitingForResponse)
      (Widget|RemovefromParent (Variables|Default|GetdialogueWidg))
      (Variables|/Game/Blueprints/Timer_Blueprint.Timer_Blueprint_C|SetTime _timer_blueprint (- (Variables|/Game/Blueprints/Timer_Blueprint.Timer_Blueprint_C|GetTime _timer_blueprint) 10))
      (Variables|Default|SetwaitingForResponse false)
      (if (< (stale Input|ActionEvents|InputActionYes _output_get) 3)
        (Utilities|FlowControl|Delay 1e+01)
        (CallFunction|GiveDemand)))))

(fn ConstructionScript)

(fn CheckConstraints
  (for _array_element (Variables|Default|Getconsts)
    (bind _foundflaw (Default|CheckItems _array_element))
    (if _foundflaw
      (Development|PrintString "game over")
      (Default|GameOver (Variables|Default|Getspawnboi)))))