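; Hitbox actor owned by an Items_Blueprint that detects what the item lands on and transfers weight to the item below.
; Construction disables collision and caches the owning item.
; Overlapping another item records it as ItemBelow, notifies the owner and stops it, while any other actor except the owner's CenterBox only stops it.
; ApplyWeight reduces the lower item's durability by only the change since the last applied weight.
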(event Custom|ApplyWeight
  (params (NewWeightApplied :type Float%20%28single-precision%29))
  (bind _itembelow (Variables|Default|GetItemBelow))
  ;[1 1 1] Add Weight to block below
  (if (not (== _itembelow (Variables|Default|GetItemNull)))
    (Default|ReduceDurability _itembelow (- NewWeightApplied (Variables|Default|GetWeightApplied)))
    (Variables|Default|SetWeightApplied NewWeightApplied)))

(event EventBeginPlay)

(event Collision|EventActorBeginOverlap
  (params (OtherActor :type Actor%20Object%20Reference))
  (bind _item (Variables|Default|GetItem))
  ;[1 1 1] Hit Something
  (bind _asitems_blueprint (Utilities|Casting|CastToItems_Blueprint OtherActor)
    (:then
      (Utilities|IsValid _item
        (:Is%20Valid
          (if (not (== _asitems_blueprint _item))
            (Variables|Default|SetItemBelow _asitems_blueprint)
            (Default|HitboxHitSomething _item)
            (Default|StopBlock _item :!label _label)))))
    (:CastFailed
      (if (not (== OtherActor (Variables|/Game/Blueprints/Items_Blueprint.Items_Blueprint_C|GetCenterBox _item)))
        (goto _label)))))

(event EventTick
  (params (DeltaSeconds :type Float%20%28single-precision%29)))

(fn ConstructionScript
  (Collision|SetCollisionEnabled (Variables|Default|GetCollisionComponent) "NoCollision")
  (bind _asitems_blueprint (Utilities|Casting|CastToItems_Blueprint (Components|GetOwner self)))
  (Variables|Default|SetItem _asitems_blueprint))

(fn ReturnItemBelowbyRef
  (return (Variables|Default|GetItemBelow)))